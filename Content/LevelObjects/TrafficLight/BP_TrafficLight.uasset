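; Traffic light level object with red, amber and green lamps whose brightness is set individually.
; BeginPlay creates three dynamic instances of TrafficLightEmmision, tints each one and assigns it to its own material slot on the TrafficLight mesh.
; The SetColour event drives each instance's Brightness parameter; BeginPlay calls it with red and green lit, amber off.
; The file contains no timing or sequencing logic.
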(event `self.ReceiveBeginPlay`
  (bind _trafficlight (`self.TrafficLight`))
  (`|ExecutionSequence`
    (:`then_0`
      (bind _returnvalue (`KismetMaterialLibrary.CreateDynamicMaterialInstance` "/Game/LevelObjects/TrafficLight/TrafficLightEmmision.TrafficLightEmmision"))
      (bind _output_get (set `self.Red` _returnvalue))
      (`MaterialInstanceDynamic.SetVectorParameterValue` _output_get "Colour" (struct :`R` 1.0 :`A` 1.0))
      (`PrimitiveComponent.SetMaterial` _trafficlight 4 _output_get))
    (:`then_1`
      (bind _returnvalue_2 (`KismetMaterialLibrary.CreateDynamicMaterialInstance` "/Game/LevelObjects/TrafficLight/TrafficLightEmmision.TrafficLightEmmision"))
      (bind _output_get_2 (set `self.Amber` _returnvalue_2))
      (`MaterialInstanceDynamic.SetVectorParameterValue` _output_get_2 "Colour" (struct :`R` 1.0 :`G` 0.773908 :`A` 1.0))
      (`PrimitiveComponent.SetMaterial` _trafficlight 3 _output_get_2))
    (:`then_2`
      (bind _returnvalue_3 (`KismetMaterialLibrary.CreateDynamicMaterialInstance` "/Game/LevelObjects/TrafficLight/TrafficLightEmmision.TrafficLightEmmision"))
      (bind _output_get_3 (set `self.Green` _returnvalue_3))
      (`MaterialInstanceDynamic.SetVectorParameterValue` _output_get_3 "Colour" (struct :`G` 1.0 :`A` 1.0))
      (`PrimitiveComponent.SetMaterial` _trafficlight 5 _output_get_3))
    (:`then_3`
      (`self.SetColour` 1.0 0.0 1.0))))

(event `SetColour`
  (params (Red :type "Float (double-precision)") (Amber :type "Float (double-precision)") (Green :type "Float (double-precision)"))
  (`MaterialInstanceDynamic.SetScalarParameterValue` (`self.Red`) "Brightness" Red)
  (`MaterialInstanceDynamic.SetScalarParameterValue` (`self.Amber`) "Brightness" Amber)
  (`MaterialInstanceDynamic.SetScalarParameterValue` (`self.Green`) "Brightness" Green))

(fn `UserConstructionScript`)